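; BP_Bar is a player-controlled bar actor that slides along the world X axis.
; BeginPlay adds the IMC_Keyboard Enhanced Input mapping context, and IA_Move stores its value in MoveValue.
; Tick moves the bar by MoveValue, MoveSpeed and delta time, clamps X symmetrically to MoveLimit, then zeroes MoveValue so motion stops when input stops.
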(event Input|EnhancedActionEvents|EnhancedInputActionIA_Move
  (params (ActionValue :type Float%20%28double-precision%29) (ElapsedSeconds :type Float%20%28double-precision%29) (TriggeredSeconds :type Float%20%28double-precision%29) (InputAction :type Input%20Action%20Object%20Reference :default "/Game/Input/IA_Move.IA_Move"))
  ;[1 1 1] 入力を設定する
  (:Triggered
    (Variables|Default|SetMoveValue ActionValue)))

(event EventBeginPlay
  ;[1 1 1] 入力を設定する
  (Input|AddMappingContext (PlayerController|LocalPlayerSubsystems|GetEnhancedInputLocalPlayerSubsystem (Game|GetPlayerController 0)) "/Game/Input/IMC_Keyboard.IMC_Keyboard" 0 "(bIgnoreAllPressedKeysUntilRelease=True,bForceImmediately=False)"))

(event Collision|EventActorBeginOverlap
  (params (OtherActor :type Actor%20Object%20Reference)))

(event EventTick
  (params (DeltaSeconds :type Float%20%28single-precision%29))
  (bind _returnvalue (Transformation|GetActorLocation))
  (bind _movelimit (Variables|Default|GetMoveLimit))
  ;[1 1 1] 移動する
  (Transformation|SetActorLocation (Math|Vector|MakeVector (Math|Float|Clamp(Float) (+ (.x _returnvalue) (* DeltaSeconds (Variables|Default|GetMoveValue) (Variables|Default|GetMoveSpeed))) (* _movelimit -1.0) _movelimit) (.y _returnvalue) (.z _returnvalue)) false false)
  (Variables|Default|SetMoveValue 0.0))

(fn ConstructionScript)