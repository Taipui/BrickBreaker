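; Ball actor for a block-breaker style game that moves, scores block hits and signals game over.
; While playing, Tick moves it along Direction at Speed with a swept move.
; Hit hides actors tagged Block, raises the score and calls UpdateScoreLabel, or calls GameOver for GameOver-tagged actors.
; A Reflect function mirrors Direction about a given normal, though nothing in this file calls it.
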(event EventBeginPlay)

(event Collision|EventHit
  (params (MyComp :type Primitive%20Component%20Object%20Reference) (Other :type Actor%20Object%20Reference) (OtherComp :type Primitive%20Component%20Object%20Reference) (bSelfMoved :type Boolean) (HitLocation :type Vector :default "0, 0, 0") (HitNormal :type Vector :default "0, 0, 0") (NormalImpulse :type Vector :default "0, 0, 0") (Hit :type Hit%20Result%20Structure%20%28by%20ref%29))
  (bind _returnvalue (Components|GetOwner OtherComp))
  (bind _score (Variables|Default|GetScore))
  (if (Actor|ActorHasTag _returnvalue "Block")
    (Rendering|SetActorHiddenInGame _returnvalue true)
    ;[1 1 1] スコア100ずつ加算
    (Math|Integer|IncrementInt _score
      (:%20%20
        (Default|CallUpdateScoreLabel (Utilities|String|Append "Score: " (Utilities|String|ToString(Integer) (* _score 100))))))
    (else
      ;[1 1 1] GameOverの処理
      (if (Actor|ActorHasTag _returnvalue "GameOver")
        (Default|CallGameOver)))))

(event EventTick
  (params (DeltaSeconds :type Float%20%28single-precision%29))
  (if (Variables|Default|GetIsPlaying)
    (Transformation|SetActorLocation (+ (* DeltaSeconds (Variables|Default|GetDirection) (Variables|Default|GetSpeed)) (Transformation|GetActorLocation)) true false)))

(fn ConstructionScript)

(fn Reflect
  (params (InNormal :type Vector))
  (Variables|Default|SetDirection (Math|Vector|MirrorVectorbyNormal (Variables|Default|GetDirection) InNormal)))